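; A platform that turns to glass on a timer and kills a non-shadow ThirdPersonCharacter that hits it in that state.
; Tick drives chained Delays that call Glass, then Normalize, though the event restoring the pulsing hex-tile material is named Normal.
; Glass and Normal swap the mesh material and set the GlassPlat flag.
; The mesh's hit event checks that flag and IsShadow before setting PlayerDead on the character.
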(event OnComponentHit(StaticMesh)
  (params (HitComponent :type Primitive%20Component%20Object%20Reference) (OtherActor :type Actor%20Object%20Reference) (OtherComp :type Primitive%20Component%20Object%20Reference) (NormalImpulse :type Vector :default "0, 0, 0") (Hit :type Hit%20Result%20Structure%20%28by%20ref%29))
  (bind _asthird_person_character (Utilities|Casting|CastToThirdPersonCharacter OtherActor))
  (if (not (Variables|/Game/ThirdPersonBP/Blueprints/ThirdPersonCharacter.ThirdPersonCharacter_C|GetisShadow _asthird_person_character))
    (if (Variables|Default|GetglassPlat)
      (Variables|/Game/ThirdPersonBP/Blueprints/ThirdPersonCharacter.ThirdPersonCharacter_C|SetplayerDead _asthird_person_character true))))

(event Custom|Glass
  (Rendering|Material|SetMaterial (Variables|Default|GetStaticMesh) 0 "/Game/StarterContent/Props/Materials/M_StatueGlass.M_StatueGlass")
  (Variables|Default|SetglassPlat true))

(event Custom|Normal
  (Rendering|Material|SetMaterial (Variables|Default|GetStaticMesh) 0 "/Game/StarterContent/Materials/M_Tech_Hex_Tile_Pulse.M_Tech_Hex_Tile_Pulse")
  (Variables|Default|SetglassPlat false))

(event EventBeginPlay)

(event Collision|EventActorBeginOverlap
  (params (OtherActor :type Actor%20Object%20Reference)))

(event EventTick
  (params (DeltaSeconds :type Float%20%28single-precision%29))
  (Utilities|FlowControl|Delay 5.0)
  (CallFunction|Glass)
  (Utilities|FlowControl|Delay 3.0)
  (CallFunction|Normal))

(fn ConstructionScript)