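; Platform actor that alternates between a normal tech-tile state and a deadly lava state.
; Tick drives a repeating timed swap through chained Delay nodes rather than timers.
; The Lava and Normal events set the mesh material and state flags.
; On mesh hit, a ThirdPersonCharacter is marked dead if the platform is lava, unless the character is in rock form.
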(event OnComponentHit(StaticMesh)
  (params (HitComponent :type Primitive%20Component%20Object%20Reference) (OtherActor :type Actor%20Object%20Reference) (OtherComp :type Primitive%20Component%20Object%20Reference) (NormalImpulse :type Vector :default "0, 0, 0") (Hit :type Hit%20Result%20Structure%20%28by%20ref%29))
  (bind _asthird_person_character (Utilities|Casting|CastToThirdPersonCharacter OtherActor))
  (if (not (Variables|/Game/ThirdPersonBP/Blueprints/ThirdPersonCharacter.ThirdPersonCharacter_C|GetisRock _asthird_person_character))
    (if (Variables|Default|GetlavaPlat)
      (Variables|/Game/ThirdPersonBP/Blueprints/ThirdPersonCharacter.ThirdPersonCharacter_C|SetplayerDead _asthird_person_character true))))

(event Custom|Lava
  (Rendering|Material|SetMaterial (Variables|Default|GetStaticMesh) 0 "/Game/lava.lava")
  (Variables|Default|SetlavaPlat true)
  (Variables|Default|SetnormalPlat false))

(event Custom|Normal
  (Rendering|Material|SetMaterial (Variables|Default|GetStaticMesh) 0 "/Game/StarterContent/Materials/M_Tech_Hex_Tile_Pulse.M_Tech_Hex_Tile_Pulse")
  (Variables|Default|SetlavaPlat false)
  (Variables|Default|SetnormalPlat true))

(event EventBeginPlay)

(event Collision|EventActorBeginOverlap
  (params (OtherActor :type Actor%20Object%20Reference)))

(event EventTick
  (params (DeltaSeconds :type Float%20%28single-precision%29))
  (Utilities|FlowControl|Delay 5.0)
  (CallFunction|Lava)
  (Utilities|FlowControl|Delay 3.0)
  (CallFunction|Normal))

(fn ConstructionScript)